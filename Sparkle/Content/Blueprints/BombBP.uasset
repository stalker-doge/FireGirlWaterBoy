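; BombBP is a bomb actor that spawns colored wire segment actors at startup.
; Shortly after BeginPlay, it loops over WireArray and calls a spawn function for each blue, red, green, white or gold entry.
; Each function reads the count at the same index in WireCutArray and spawns that many segments of its color, all at the bomb's own transform.
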(event EventBeginPlay
  (Utilities|FlowControl|Delay 0.2)
  (for (_array_element _array_index) (Variables|Default|GetwireArray)
    (switch string _array_element
      (:BLUE%20Wire
        (|SpawnBlue _array_index))
      (:RED%20Wire
        (|SpawnRed _array_index))
      (:GREEN%20Wire
        (|SpawnGreen _array_index))
      (:WHITE%20Wire
        (|SpawnWhite _array_index))
      (:GOLD%20Wire
        (|SpawnGold _array_index)))))

(event Collision|EventActorBeginOverlap
  (params (OtherActor :type Actor%20Object%20Reference)))

(event EventTick
  (params (DeltaSeconds :type Float%20%28single-precision%29)))

(fn ConstructionScript)